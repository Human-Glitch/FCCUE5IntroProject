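; BP_PlayerController is a player controller that owns the player's HUD and sets gameplay input mode.
; On BeginPlay it creates the BP_HUD widget, adds it to the viewport, switches to game-only input and hides the mouse cursor.
; UpdateHealth pushes a new health value into the HUD's bar, scaled from a 100-point range, and its formatted text.
; A GetSensitivity function exposes the stored Sensitivity value.
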(event Custom|CreateHUD
  (bind _returnvalue (UserInterface|CreateWidget "/Game/UI/HUD/BP_HUD.BP_HUD_C"))
  (bind _output_get (Variables|Default|SetHUD _returnvalue))
  (UserInterface|Viewport|AddtoViewport _output_get 0))

(event Custom|UpdateHealth
  (params (NewHealth :type Float%20%28double-precision%29))
  (bind _hud (Variables|Default|GetHUD))
  (Progress|SetPercent (Variables|/Game/UI/HUD/BP_HUD.BP_HUD_C|GetHealthBar _hud) (/ NewHealth 1e+02))
  (Rendering|Components|TextRender|SetText (Variables|/Game/UI/HUD/BP_HUD.BP_HUD_C|GetHealthText _hud) (Utilities|Text|FormatText "+{Health}" NewHealth)))

(event EventBeginPlay
  (CallFunction|CreateHUD)
  (Input|SetInputModeGameOnly self false)
  (Variables|Default|SetbShowMouseCursor false))

(event EventTick
  (params (DeltaSeconds :type Float%20%28single-precision%29)))

(fn ConstructionScript)

(fn GetSensitivity
  (return (Variables|Default|GetSensitivity)))