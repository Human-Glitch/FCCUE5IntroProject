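; Vector2 is a Blueprint object that wraps a two-component X/Y vector.
; Getters return each component or both together, and SetVector2 writes both from its inputs.
; SetX and SetY take no inputs as shown and assign each component to itself.
; PrintVector2 prints both components as a labelled string, using the object's outer as world context.
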(fn GetX
  (return (Variables|Default|GetX)))

(fn GetY
  (return (Variables|Default|GetY)))

(fn SetX
  (Variables|Default|SetX (Variables|Default|GetX))
  (return))

(fn SetY
  (Variables|Default|SetY (Variables|Default|GetY))
  (return))

(fn GetVector2
  (return (Variables|Default|GetX) (Variables|Default|GetY)))

(fn SetVector2
  (params (X :type Float%20%28double-precision%29) (Y :type Float%20%28double-precision%29))
  (Variables|Default|SetX X)
  (Variables|Default|SetY Y)
  (return))

(fn PrintVector2
  (Development|PrintString (Utilities|GetOuterObject self) (Utilities|String|Append "X:" (Utilities|String|ToString(Float) (Variables|Default|GetX)) "Y:" (Utilities|String|ToString(Float) (Variables|Default|GetY)))))