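; Player character with axis-driven movement and look, plus pickup and physics-nudge interactions.
; A looping timer polls for BP_PlayerController to cache sensitivity and push health, while BeginPlay also spawns a test-style BP_Pickup.
; Overlaps track nearby actors for Interact, which destroys the pickup and subtracts health, quitting the game at zero, or applies a forward impulse to the InteractionActor.
; Left click runs a debug-drawn camera trace that destroys hit pickups.
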(event EventBeginPlay
  ;[1 1 1] Polling for References
  (bind _returnvalue (Utilities|Time|SetTimerbyFunctionName 0 "Initialize" 0.01 true))
  (Variables|Default|SetInitializeTimer _returnvalue)
  (Game|SpawnActorfromClass "/Game/Blueprints/BP_Pickup.BP_Pickup_C" (Math|Transform|MakeTransform "5770.000000,-1980.000000,110.000000" "0, 0, 0" "1.000000,1.000000,1.000000") "Undefined" "MultiplyWithRoot" 0 9e+01 0))

(event Collision|EventActorBeginOverlap
  (params (OtherActor :type Actor%20Object%20Reference))
  (bind _asbp_pickup (Utilities|Casting|CastToBP_Pickup OtherActor)
    (:then
      (Variables|Default|SetNearbyPickup _asbp_pickup))
    (:CastFailed
      (bind _asinteraction_actor (Utilities|Casting|CastToInteractionActor OtherActor))
      (Variables|Default|SetInteractionActor _asinteraction_actor))))

(event Collision|EventActorEndOverlap
  (params (OtherActor :type Actor%20Object%20Reference))
  (bind _asbp_pickup (Utilities|Casting|CastToBP_Pickup OtherActor)
    (:then
      (if (== _asbp_pickup (Variables|Default|GetNearbyPickup))
        (Variables|Default|SetNearbyPickup 0)))
    (:CastFailed
      (bind _asinteraction_actor (Utilities|Casting|CastToInteractionActor OtherActor))
      (if (== _asinteraction_actor (Variables|Default|GetInteractionActor))
        (Variables|Default|SetInteractionActor 0)))))

(event Input|ActionEvents|InputActionInteract
  (params (Key :type Key%20Structure :default "None"))
  (:Pressed
    (Utilities|FlowControl|Sequence
      (:then_0
        (CallFunction|Pickup))
      (:then_1
        (CallFunction|NudgeBall)))))

(event Input|AxisEvents|InputAxisMoveForwardBackward
  (params (AxisValue :type Float%20%28single-precision%29))
  ;[1 1 1] Movement and Camera
  (Pawn|Input|AddMovementInput (Transformation|GetActorForwardVector) AxisValue false))

(event Input|AxisEvents|InputAxisMoveHorizontal
  (params (AxisValue :type Float%20%28single-precision%29))
  ;[1 1 1] Movement and Camera
  (Pawn|Input|AddMovementInput (Transformation|GetActorRightVector) AxisValue false))

(event Input|AxisEvents|InputAxisLookAround
  (params (AxisValue :type Float%20%28single-precision%29))
  ;[1 1 1] Movement and Camera
  (Pawn|Input|AddControllerYawInput (* AxisValue (Variables|Default|GetSensitivity))))

(event Input|AxisEvents|InputAxisLookUp
  (params (AxisValue :type Float%20%28single-precision%29))
  ;[1 1 1] Movement and Camera
  (Pawn|Input|AddControllerPitchInput (* AxisValue (Variables|Default|GetSensitivity))))

(event Input|MouseEvents|LeftMouseButton
  (params (Key :type Key%20Structure :default "None"))
  (bind _returnvalue (Game|GetPlayerCameraManager 0))
  (bind _returnvalue_2 (Transformation|GetActorLocation _returnvalue))
  (:Pressed
    (bind _outhit (Collision|LineTraceByChannel _returnvalue_2 (+ _returnvalue_2 (* (Transformation|GetActorForwardVector _returnvalue) 5e+04)) "TraceTypeQuery1" false 0 "ForDuration"))
    (Rendering|Debug|DrawDebugSphere (.location _outhit) 5e+01 20 "(R=0.289657,G=1.000000,B=0.349899,A=1.000000)" 1e+01 2.0)
    (bind _asbp_pickup (Utilities|Casting|CastToBP_Pickup (.hitactor _outhit)))
    (Actor|DestroyActor _asbp_pickup)))

(fn ConstructionScript)

(fn Initialize
  (bind _returnvalue (Game|GetPlayerController 0))
  (bind _asbp_player_controller (Utilities|Casting|CastToBP_PlayerController _returnvalue))
  (Utilities|IsValid _asbp_player_controller
    (:Is%20Valid
      (bind _output_get (Variables|Default|SetPCref _asbp_player_controller))
      (Variables|Default|SetSensitivity (Default|GetSensitivity _output_get))
      (Default|UpdateHealth (Variables|Default|GetPCref) (Variables|Default|GetHealth))
      (Utilities|Time|ClearandInvalidateTimerbyHandle (Variables|Default|GetInitializeTimer)))
    (:Is%20Not%20Valid
      (Development|PrintString "Player Controller is not valid."))))

(fn Pickup
  (bind _nearbypickup (Variables|Default|GetNearbyPickup)
    (:then
      (Development|PrintString (Utilities|String|ToString(Float) (Variables|/Game/Blueprints/BP_Pickup.BP_Pickup_C|GetHealthPoints _nearbypickup)))
      (Actor|DestroyActor _nearbypickup)
      (Variables|Default|SetNearbyPickup (.AsBP%20Pickup (Utilities|Casting|CastToBP_Pickup (Utilities|Array|Get(acopy) (Collision|GetOverlappingActors "/Game/Blueprints/BP_Pickup.BP_Pickup_C" :!class /Script/Engine.Actor)))))
      (CallFunction|SetHealth (- (Variables|Default|GetHealth) 4e+01)))
    (:else)))

(fn NudgeBall
  (bind _interactionactor (Variables|Default|GetInteractionActor)
    (:then
      (Physics|AddImpulse (Variables|/Game/Blueprints/InteractionActor.InteractionActor_C|GetStaticMesh _interactionactor) (* (Transformation|GetActorForwardVector) 1e+04) "None" false))
    (:else)))

(fn SetHealth
  (params (Health :type Float%20%28double-precision%29))
  (bind _output_get (Variables|Default|SetHealth Health))
  (if (<= _output_get 0.0)
    (Development|ExecuteConsoleCommand "exit" 0)
    (else
      (Default|UpdateHealth (Variables|Default|GetPCref) (Variables|Default|GetHealth)))))